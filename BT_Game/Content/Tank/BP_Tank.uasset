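; BP_Tank is a tank pawn that wires player input to its aiming and movement components.
; On BeginPlay it hands the barrel and turret to TankAiming and the left and right tracks to TankMovement.
; Forward and turn axes send movement intents to TankMovement, and the Fire action calls TankAiming.
; Aim axes rotate the camera's azimuth gimbal and spring arm, scaled by delta time.
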(event `self.ReceiveBeginPlay`
  (`TankAimingComponent.Initialise` (`self.TankAiming`) (`self.Barrel`) (`self.TankTurret`))
  (`TankMovementComponent.Initialise` (`self.TankMovement`) (`self.LeftTrack`) (`self.RightTrack`)))

(event `InputAxis|AimAzimuth`
  (params (AxisValue :type "Float (single-precision)"))
  ;[1 1 1] Input Gouing
  (`SceneComponent.K2_AddLocalRotation` (`self.Azimuth Gimbal`) (`KismetMathLibrary.MakeRotator` 0.0 0.0 (* AxisValue (`GameplayStatics.GetWorldDeltaSeconds`))) false false))

(event `InputAxis|Forward`
  (params (AxisValue :type "Float (single-precision)"))
  ;[1 1 1] Tracks throttle
  (`TankMovementComponent.IntendMoveForward` (`self.TankMovement`) AxisValue))

(event `InputAxis|Move Right`
  (params (AxisValue :type "Float (single-precision)"))
  ;[1 1 1] Tracks throttle
  (`TankMovementComponent.IntendRotateRight` (`self.TankMovement`) AxisValue))

(event `InputAxis|AimElevate`
  (params (AxisValue :type "Float (single-precision)"))
  ;[1 1 1] Input Gouing
  (`SceneComponent.K2_AddLocalRotation` (`self.SpringArm`) (`KismetMathLibrary.MakeRotator` 0.0 (* AxisValue (`GameplayStatics.GetWorldDeltaSeconds`))) false false))

(event `InputAction|Fire`
  (params (Key :type "Key Structure" :default "AnyKey"))
  ;[1 1 1] Input Gouing
  (:`Pressed`
    (`TankAimingComponent.Fire` (`self.TankAiming`))))

(fn `NewFunction_0`)

(fn `UserConstructionScript`)